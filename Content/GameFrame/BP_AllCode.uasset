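; BP_AllCode is a reference Blueprint cataloguing a WebSocket subsystem's API for server and client connections.
; One graph holds unwired calls for starting, stopping, linking, unlinking and sending messages on a local port.
; Server and client delegate graphs pair bind and unbind calls with events that print connect, error, message and close details.
; None of the subsystem calls is connected to an execution path, so they never run.
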(fn ConstructionScript)

(event Custom|ServerConnectSuccess
  (params (ServerConnectionID :type Guid%20Structure) (ClientConnectionID :type Guid%20Structure))
  (Development|PrintString (Utilities|String|Append "--ServerConnect Success" "--ServerConnectionID:" (Guid|ToString(Guid) ServerConnectionID) "--ClientConnectionID:" (Guid|ToString(Guid) ClientConnectionID))))

(event Custom|ServerConnectFail
  (params (ServerConnectionID :type Guid%20Structure))
  (Development|PrintString (Utilities|String|Append "--ServerConnect Error" "--ServerConnectionID:" (Guid|ToString(Guid) ServerConnectionID))))

(event Custom|ServerReceiveMessage
  (params (ServerConnectionID :type Guid%20Structure) (Message :type String))
  (Development|PrintString (Utilities|String|Append "--ServerConnect Message" "--ServerConnectionID:" (Guid|ToString(Guid) ServerConnectionID) "--ServerMessage::" Message)))

(event Custom|ServerConnectClose
  (params (ServerConnectionID :type Guid%20Structure))
  (Development|PrintString (Utilities|String|Append "--ServerConnectClose" "--ServerConnectionID:" (Guid|ToString(Guid) ServerConnectionID))))

(event Custom|ClientConnectSuccess
  (params (ServerConnectionID :type Guid%20Structure) (ClientConnectionID :type Guid%20Structure))
  (Development|PrintString (Utilities|String|Append "--ClientConnect Success" "--ClientConnectionID:" (Guid|ToString(Guid) ServerConnectionID) "--ClientConnectionID:" (Guid|ToString(Guid) ClientConnectionID))))

(event Custom|ClientConnectError
  (params (ErrorMessage :type String) (ClientConnectionID :type Guid%20Structure))
  (Development|PrintString (Utilities|String|Append "--ClientConnectError:" "--ClientConnectionID:" (Guid|ToString(Guid) ClientConnectionID))))

(event Custom|ClientReceiveMessage
  (params (ClientConnectionID :type Guid%20Structure) (Message :type String))
  (Development|PrintString (Utilities|String|Append "--Client Receive Message" "--ClientConnectionID:" (Guid|ToString(Guid) ClientConnectionID) "--ClientMessage::" Message)))

(event Custom|ClientConnectClose
  (params (StatusCode :type Integer) (Reason :type String) (bWasClean :type Boolean) (ClientConnectionID :type Guid%20Structure))
  (Development|PrintString (Utilities|String|Append "--Client Connect Close" "--ClientConnectionID:" (Guid|ToString(Guid) ClientConnectionID))))